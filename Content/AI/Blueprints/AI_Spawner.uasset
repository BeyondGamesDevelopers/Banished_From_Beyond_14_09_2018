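; AI spawner actor that places a Banished AI character in the level when play begins.
; Its AIType selects the behavior tree, with only Aggressive assigned one, and is copied onto the spawned character.
; Spawn location and rotation come from Get Spawn Transform, whose graph contains only unconnected nodes.
; The construction script colors the arrow and cube grid material by AIType as a visual marker.
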(event `self.ReceiveBeginPlay`
  (bind (_location _rotation) (`self.Get Spawn Transform`))
  (bind _returnvalue (`AIBlueprintHelperLibrary.SpawnAIFromClass` "/Game/AI/Blueprints/Banished_AI_Character.Banished_AI_Character_C" (select `/Game/AI/Blueprints/AIType` (`self.AIType`) :`NewEnumerator2` "/Game/AI/AI_BT_Aggressive.AI_BT_Aggressive" :!type "BehaviorTree Object Reference") _location _rotation true))
  (bind _asbanished_ai_character (cast `/Game/AI/Blueprints/Banished_AI_Character` _returnvalue))
  (set `/Game/AI/Blueprints/Banished_AI_Character.AIType` (`self.AIType`) _asbanished_ai_character))

(fn `UserConstructionScript`
  (bind _colour (`self.Colour`))
  (switch `/Game/AI/Blueprints/AIType` (`self.AIType`)
    (:`NewEnumerator0`
      (set `self.Colour` (struct :`G` 1.0 :`A` 1.0)))
    (:`NewEnumerator1`
      (set `self.Colour` (struct :`B` 1.0 :`A` 1.0)))
    (:`NewEnumerator2`
      (set `self.Colour` (struct :`R` 1.0 :`A` 1.0))))
  (`ArrowComponent.SetArrowColor` (`self.Arrow`) _colour)
  (`MeshComponent.SetVectorParameterValueOnMaterials` (`self.Cube`) "GridColor" (* (`KismetMathLibrary.Conv_LinearColorToVector` _colour) 0.5)))