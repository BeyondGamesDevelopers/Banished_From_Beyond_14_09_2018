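; AI controller for Banished AI characters that feeds perception results to a blackboard and selects a behavior tree by AI type, with only Aggressive assigned.
; Perception updates track seen and heard actors, gating per-tick player checks for noise and distance-weighted visibility with a close-range boost.
; When the player is barely detected, tagged actors' stimuli become averaged locations and a suspicion flag.
; Tick also syncs AI state and Veil strength.
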(event `self.OnPossess`
  (params (PossessedPawn :type "Pawn Object Reference"))
  ;[0 1 0] Event Possessed
  (`self.UseBlackboard` "/Game/AI/AI_BB.AI_BB")
  (`self.RunBehaviorTree` (select `/Game/AI/Blueprints/AIType` (`/Game/AI/Blueprints/Banished_AI_Character.AIType` (cast `/Game/AI/Blueprints/Banished_AI_Character` PossessedPawn :!pure true)) :`NewEnumerator2` "/Game/AI/AI_BT_Aggressive.AI_BT_Aggressive" :!type "BehaviorTree Object Reference"))
  (`self.Set References` PossessedPawn)
  (`self.Possession` PossessedPawn))

(event `self.OnUnpossess`
  (params (UnpossessedPawn :type "Pawn Object Reference"))
  ;[0 1 0] Event Unpossessed
  (`self.DebugLog` UnpossessedPawn))

(event `Deactivate AI Controller`
  ;[0 1 0] Deactivate AI Controller
  (`self.Deactivate Controller`))

(event `self.ReceiveTick`
  (params (DeltaSeconds :type "Float (single-precision)"))
  (bind _controlledpawn (`self.ControlledPawn`))
  (bind _controlledpawn_2 (`self.ControlledPawn`))
  ;[1 0 0] Increase FPS OPTIMIZE!
  (`/Engine/EditorBlueprintResources/StandardMacros.IsValid` _controlledpawn
    (:`Is Valid`
      (if (and (`KismetSystemLibrary.IsValid` _controlledpawn) (`KismetSystemLibrary.IsValid` (`self.Player`)) (== (`Pawn.GetController` _controlledpawn_2) self) (not (`/Game/AI/Blueprints/Banished_AI_Character.IsDead` _controlledpawn_2)))
        (`self.UpdateInfo`)
        (`self.Set Enable EQS Refresh`)
        ;[0 1 0] Player Perception
        (`/Engine/EditorBlueprintResources/StandardMacros.Gate` true :!label _label
          (:`Exit`
            (`|ExecutionSequence`
              (:`then_0`
                (`self.IsPlayerSeen`))
              (:`then_1`
                (`self.IsPlayerHeard`)))))))))

(event `self.AIPerception.OnPerceptionUpdated`
  (params (UpdatedActors :type "Array of Actor Object Reference"))
  (bind _blackboard (`self.Blackboard`))
  (bind _controlledpawn (`self.ControlledPawn`))
  (`/Engine/EditorBlueprintResources/StandardMacros.IsValid` (`self.ControlledPawn`)
    (:`Is Valid`
      (if (and (`KismetSystemLibrary.IsValid` (`self.ControlledPawn`)) (`KismetSystemLibrary.IsValid` (`self.Player`)) (== (`Pawn.GetController` _controlledpawn) self) (not (`/Game/AI/Blueprints/Banished_AI_Character.IsDead` _controlledpawn)))
        (`self.Update Percieved Actors` UpdatedActors)
        (`|ExecutionSequence`
          (:`then_0`
            ;[0 1 0] Player Perception
            (if (`KismetArrayLibrary.Array_Contains` (`self.PercievedActors`) (`self.Player`))
              (goto _label :!via `Open`)
              (else
                (`self.Ignore Player`)
                (goto _label :!via `Close`))))
          (:`then_1`
            ;[0 1 0] General Perception
            (if (and (< (`BlackboardComponent.GetValueAsFloat` _blackboard "PercievedPlayerVisibility") 0.5) (not (`BlackboardComponent.GetValueAsBool` _blackboard "PercievedPlayerNoise")) (not (`BlackboardComponent.GetValueAsBool` _blackboard "PercievedPlayerTouch")))
              (`self.Update Perception`))))))))

(fn `CalculateAverageHeardVector`
  (locals (AvgHeardVector :type "Vector Structure"))
  (bind _avgheardvector (`local.AvgHeardVector`))
  (bind _heardvectors (`/Game/AI/Blueprints/Banished_AI_Character.HeardVectors` (`self.ControlledPawn`)))
  (for _array_element _heardvectors
    (set `local.AvgHeardVector` (+ _array_element _avgheardvector)))
  (bind _output_get (set `/Game/AI/Blueprints/Banished_AI_Character.LastHeardLocation` (/ _avgheardvector (`KismetArrayLibrary.Array_Length` _heardvectors)) (`self.ControlledPawn`)))
  (`BlackboardComponent.SetValueAsVector` (`self.Blackboard`) "LastHeardLocation" _output_get)
  (set `local.AvgHeardVector` (0.0 0.0 0.0)))

(fn `CalculateAverageSeenVector`
  (locals (AvgSeenVector :type "Vector Structure"))
  (bind _avgseenvector (`local.AvgSeenVector`))
  (bind _seenvectors (`/Game/AI/Blueprints/Banished_AI_Character.SeenVectors` (`self.ControlledPawn`)))
  (for _array_element _seenvectors
    (set `local.AvgSeenVector` (+ _array_element _avgseenvector)))
  (bind _output_get (set `/Game/AI/Blueprints/Banished_AI_Character.LastSeenLocation` (/ _avgseenvector (`KismetArrayLibrary.Array_Length` _seenvectors)) (`self.ControlledPawn`)))
  (`BlackboardComponent.SetValueAsVector` (`self.Blackboard`) "LastSeenLocation" _output_get)
  (set `local.AvgSeenVector` (0.0 0.0 0.0)))

(fn `Deactivate Controller`
  (`self.UnPossess`)
  (`BrainComponent.StopLogic` (`self.BrainComponent`) "AI Is Dead")
  (`self.K2_DestroyActor`)
  ;[1 0 1] DEBUG
  (`KismetSystemLibrary.PrintString` (`KismetStringLibrary.Concat_StrStr` "DESTROYED AI CONTROLLER: " (`KismetSystemLibrary.GetDisplayName` self)) true true (struct :`R` 1.0 :`A` 1.0) 3.0))

(fn `DebugLog`
  (params (Object :type "Object Object Reference"))
  (`KismetSystemLibrary.PrintString` (`KismetStringLibrary.Concat_StrStr` (`KismetSystemLibrary.GetDisplayName` self) " UNPOSSESSED: " (`KismetSystemLibrary.GetDisplayName` Object)) true true (struct :`R` 1.0 :`G` 0.069749 :`A` 1.0) 5.0))

(fn `Get Actors Perception`
  (params (`AI Perception` :type "AIPerceptionComponent Object Reference") (Actor :type "Actor Object Reference") (SenseIndex :type Integer))
  (returns (`Target Actor` :type "Actor Object Reference") (Blackboard :type "BlackboardComponent Object Reference") (LastSensedStimuli :type "Array of AIStimulus Structure") (Age :type "Float (double-precision)") (`Expiration Age` :type "Float (double-precision)") (Strength :type "Float (double-precision)") (`Stimulus Location` :type "Vector Structure") (`Receiver Location` :type "Vector Structure") (Tag :type Name) (`Successfully Sensed` :type Boolean))
  (bind _info (`AIPerceptionComponent.GetActorsPerception` `AI Perception` Actor))
  (bind (_target _lastsensedstimuli) (break `ActorPerceptionBlueprintInfo` _info))
  (bind (_age _expirationage _strength _stimuluslocation _receiverlocation _tag _bsuccessfullysensed) (break `AIStimulus` (`|GetArrayItem` _lastsensedstimuli SenseIndex)))
  (return _target (`self.Blackboard`) _lastsensedstimuli _age _expirationage _strength _stimuluslocation _receiverlocation _tag _bsuccessfullysensed))

(fn `Ignore Player`
  (bind _blackboard (`self.Blackboard`))
  (`BlackboardComponent.SetValueAsFloat` _blackboard "PercievedPlayerVisibility" 0.0)
  (`BlackboardComponent.SetValueAsBool` _blackboard "PercievedPlayerNoise" false)
  (set `/Game/Player/Blueprints/Banished_Player.InEnemyLightRange` false (`self.Player`)))

(fn `IsPlayerHeard`
  (bind (_target_actor _blackboard _lastsensedstimuli _age _expiration_age _strength _stimulus_location _receiver_location _tag _successfully_sensed) (`self.Get Actors Perception` (`self.AIPerception`) (`self.Player`) 1))
  (`BlackboardComponent.SetValueAsBool` (`self.Blackboard`) "PercievedPlayerNoise" _successfully_sensed)
  (if _successfully_sensed
    (bind _output_get (set `/Game/AI/Blueprints/Banished_AI_Character.LastHeardLocation` _stimulus_location (`self.ControlledPawn`)))
    (`BlackboardComponent.SetValueAsVector` (`self.Blackboard`) "LastHeardLocation" _output_get)))

(fn `IsPlayerSeen`
  (bind _blackboard (`self.Blackboard`))
  (bind _max_close_perception_radius (`self.Max Close Perception Radius`))
  (bind _min_close_perception_radius (`self.Min Close Perception Radius`))
  (bind _controlledpawn (`self.ControlledPawn`))
  (bind _player (`self.Player`))
  (bind _returnvalue (`KismetMathLibrary.NormalizeToRange` (`KismetMathLibrary.FClamp` (`self.GetDistanceTo` _controlledpawn _player) _min_close_perception_radius _max_close_perception_radius) _min_close_perception_radius _max_close_perception_radius))
  (bind _returnvalue_2 (<= _returnvalue 0.5))
  (bind _returnvalue_3 (* (`self.PlayerVisibility`) (`KismetMathLibrary.InverseLerp` 1.0 0.0 (`KismetMathLibrary.NormalizeToRange` (`KismetMathLibrary.FClamp` (`self.GetDistanceTo` _controlledpawn _player) 0.0 2500.0) 0.0 2500.0))))
  (bind (_target_actor _blackboard_2 _lastsensedstimuli _age _expiration_age _strength _stimulus_location _receiver_location _tag _successfully_sensed) (`self.Get Actors Perception` (`self.AIPerception`) (`self.Player`)))
  (if _successfully_sensed
    (`BlackboardComponent.SetValueAsFloat` _blackboard "PercievedPlayerVisibility" (`KismetMathLibrary.SelectFloat` (`KismetMathLibrary.FClamp` (+ _returnvalue_3 (* (`KismetMathLibrary.InverseLerp` 1.0 0.0 _returnvalue) 0.7))) _returnvalue_3 _returnvalue_2))
    ;[1 0.4695 0] Results In Stuttered Draining Of Mana
    (set `/Game/Player/Blueprints/Banished_Player.InEnemyLightRange` _returnvalue_2 (`self.Player`))
    (if (>= (`BlackboardComponent.GetValueAsFloat` _blackboard "PercievedPlayerVisibility") 0.05)
      (bind _output_get (set `/Game/AI/Blueprints/Banished_AI_Character.LastSeenLocation` _stimulus_location (`self.ControlledPawn`)))
      (`BlackboardComponent.SetValueAsVector` (`self.Blackboard`) "LastSeenLocation" _output_get))))

(fn `IsPlayerTouched`
  (bind (_target_actor _blackboard _lastsensedstimuli _age _expiration_age _strength _stimulus_location _receiver_location _tag _successfully_sensed) (`self.Get Actors Perception` (`self.AIPerception`) (`self.Player`) 2))
  (`BlackboardComponent.SetValueAsBool` (`self.Blackboard`) "PercievedPlayerTouch" _successfully_sensed)
  (return))

(fn `Possession`
  (params (ControlledActor :type "Actor Object Reference"))
  (`SceneComponent.K2_SetRelativeRotation` :`self` (`/Game/AI/Blueprints/Banished_AI_Character.CameraLagParent` (`self.ControlledPawn`)))
  ;[1 0 1] DEBUG
  (`KismetSystemLibrary.PrintString` (`KismetStringLibrary.Concat_StrStr` (`KismetSystemLibrary.GetDisplayName` self) " POSSESSED: " (`KismetSystemLibrary.GetDisplayName` ControlledActor)) true true (struct :`R` 0.117607 :`G` 1.0 :`A` 1.0) 5.0))

(fn `Set Enable EQS Refresh`
  (bind _blackboard (`self.Blackboard`))
  (set `/Game/AI/Blueprints/Banished_AI_Character.EnableEQSMemoryRefresh` (and (<= (`BlackboardComponent.GetValueAsFloat` _blackboard "Suspicion") 0.0) (== (`BlackboardComponent.GetValueAsEnum` _blackboard "AIState") (enumliteral `/Game/AI/Blueprints/AIState` "NewEnumerator0")) (not (`/Game/AI/Blueprints/Banished_AI_Character.PercievedStimuli` (`self.ControlledPawn`)))) (`self.ControlledPawn`)))

(fn `Set Player`
  (bind _asbanished_game_mode (cast `/Game/Global/Framework/Banished_GameMode` (`GameplayStatics.GetGameMode`)))
  (bind _output_get (set `self.Player` (`/Game/Global/Framework/Banished_GameMode.Player` _asbanished_game_mode)))
  (`BlackboardComponent.SetValueAsObject` (`self.Blackboard`) "Player" _output_get)
  (return))

(fn `Set References`
  (params (`Possessed Pawn` :type "Pawn Object Reference"))
  (bind _asbanished_game_state (cast `/Game/Global/Framework/Banished_GameState` (`GameplayStatics.GetGameState`)))
  (set `self.GameState` _asbanished_game_state)
  (bind _asbanished_ai_character (cast `/Game/AI/Blueprints/Banished_AI_Character` `Possessed Pawn`)
    (:`then`
      (`self.SetControlledPawn` _asbanished_ai_character)
      (`self.Set Player`)
      (return))
    (:`CastFailed`
      (`KismetSystemLibrary.PrintString` "FAILED TO SET CONTROLLED PAWN" true true (struct :`R` 1.0 :`A` 1.0) 5.0))))

(fn `SetControlledPawn`
  (params (`Input Pawn` :type "/Game/AI/Blueprints/Banished_AI_Character Object Reference"))
  (bind _output_get (set `self.ControlledPawn` `Input Pawn`))
  (`BlackboardComponent.SetValueAsObject` (`self.Blackboard`) "ControlledPawn" _output_get))

(fn `SetPercievedSuspiciousStimuli`
  (params (`Percieved Stimuli` :type Boolean))
  (bind _blackboard (`self.Blackboard`))
  (bind _returnvalue (`BlackboardComponent.GetValueAsEnum` (`self.Blackboard`) "AIState"))
  (if (and `Percieved Stimuli` (or (== _returnvalue (enumliteral `/Game/AI/Blueprints/AIState` "NewEnumerator0")) (== _returnvalue (enumliteral `/Game/AI/Blueprints/AIState` "NewEnumerator6"))))
    (`BlackboardComponent.SetValueAsBool` _blackboard "PercievedSuspiciousStimuli" true)
    (else
      (`BlackboardComponent.SetValueAsBool` _blackboard "PercievedSuspiciousStimuli" false))))

(fn `SetSpawnLocation`
  (params (`Input Vector` :type "Vector Structure"))
  (bind _output_get (set `/Game/AI/Blueprints/Banished_AI_Character.SpawnLocation` `Input Vector` (`self.ControlledPawn`)))
  (`BlackboardComponent.SetValueAsVector` (`self.Blackboard`) "SpawnLocation" _output_get))

(fn `Update Perception`
  (bind _controlledpawn (`self.ControlledPawn`))
  (bind _controlledpawn_2 (`self.ControlledPawn`))
  (bind _controlledpawn_3 (`self.ControlledPawn`))
  (bind _controlledpawn_4 (`self.ControlledPawn`))
  (for _array_element (`self.PercievedActors`)
    (if (`self.ActorHasTag` _array_element "Perceivable")
      (`|ExecutionSequence`
        (:`then_0`
          (bind (_target_actor _blackboard _lastsensedstimuli _age _expiration_age _strength _stimulus_location _receiver_location _tag _successfully_sensed) (`self.Get Actors Perception` (`self.AIPerception`) _array_element))
          (if _successfully_sensed
            (if (`self.ActorHasTag` _target_actor "Visible")
              (`KismetArrayLibrary.Array_AddUnique` (`/Game/AI/Blueprints/Banished_AI_Character.SeenVectors` _controlledpawn_2) _stimulus_location)
              (`KismetArrayLibrary.Array_AddUnique` (`/Game/AI/Blueprints/Banished_AI_Character.PercievedArray` _controlledpawn_2) true :!label _label))))
        (:`then_1`
          (bind (_target_actor_2 _blackboard_2 _lastsensedstimuli_2 _age_2 _expiration_age_2 _strength_2 _stimulus_location_2 _receiver_location_2 _tag_2 _successfully_sensed_2) (`self.Get Actors Perception` (`self.AIPerception`) _array_element 1))
          (if _successfully_sensed_2
            (if (`self.ActorHasTag` _target_actor_2 "Hearable")
              (`KismetArrayLibrary.Array_AddUnique` (`/Game/AI/Blueprints/Banished_AI_Character.HeardVectors` (`self.ControlledPawn`)) _stimulus_location_2)
              (goto _label)))))))
  (bind _output_get (set `/Game/AI/Blueprints/Banished_AI_Character.SeenVectors` (`/Game/AI/Blueprints/Banished_AI_Character.SeenVectors` _controlledpawn_3) _controlledpawn_3))
  (bind _output_get_2 (set `/Game/AI/Blueprints/Banished_AI_Character.HeardVectors` (`/Game/AI/Blueprints/Banished_AI_Character.HeardVectors` _controlledpawn_3) _controlledpawn))
  (bind _output_get_3 (set `/Game/AI/Blueprints/Banished_AI_Character.PercievedArray` (`/Game/AI/Blueprints/Banished_AI_Character.PercievedArray` _controlledpawn) _controlledpawn))
  (bind _output_get_4 (set `/Game/AI/Blueprints/Banished_AI_Character.PercievedStimuli` (`KismetArrayLibrary.Array_Contains` _output_get_3 true) (`self.ControlledPawn`)))
  (`self.SetPercievedSuspiciousStimuli` _output_get_4)
  (`|ExecutionSequence`
    (:`then_0`
      (if (`KismetArrayLibrary.Array_IsValidIndex` _output_get)
        (`self.CalculateAverageSeenVector`)
        (`KismetArrayLibrary.Array_Clear` (`/Game/AI/Blueprints/Banished_AI_Character.SeenVectors` _controlledpawn_4))
        (`KismetArrayLibrary.Array_Clear` (`/Game/AI/Blueprints/Banished_AI_Character.PercievedArray` _controlledpawn_4) :!label _label_2)))
    (:`then_1`
      (if (`KismetArrayLibrary.Array_IsValidIndex` _output_get_2)
        (`self.CalculateAverageHeardVector`)
        (`KismetArrayLibrary.Array_Clear` (`/Game/AI/Blueprints/Banished_AI_Character.HeardVectors` _controlledpawn_4))
        (goto _label_2)))))

(fn `Update Percieved Actors`
  (params (`Actor Array` :type "Array of Actor Object Reference"))
  (bind _visibleactors (`self.VisibleActors`))
  (bind _heardactors (`self.HeardActors`))
  (bind _percievedactors (`self.PercievedActors`))
  (bind _aiperception (`self.AIPerception`))
  (for _array_element `Actor Array`
    (`KismetArrayLibrary.Array_Clear` (`self.PercievedActors`))
    (`|ExecutionSequence`
      (:`then_0`
        (bind (_target_actor _blackboard _lastsensedstimuli _age _expiration_age _strength _stimulus_location _receiver_location _tag _successfully_sensed) (`self.Get Actors Perception` _aiperception _array_element))
        (if _successfully_sensed
          (bind _returnvalue (`AIPerceptionSystem.GetSenseClassForStimulus` (`|GetArrayItem` _lastsensedstimuli)))
          (set `self.LastSenseClass` _returnvalue)
          (`KismetArrayLibrary.Array_AddUnique` _visibleactors _array_element)
          (else
            (`KismetArrayLibrary.Array_RemoveItem` _visibleactors _array_element))))
      (:`then_1`
        (bind (_target_actor_2 _blackboard_2 _lastsensedstimuli_2 _age_2 _expiration_age_2 _strength_2 _stimulus_location_2 _receiver_location_2 _tag_2 _successfully_sensed_2) (`self.Get Actors Perception` _aiperception _array_element 1))
        (if _successfully_sensed_2
          (bind _returnvalue_2 (`AIPerceptionSystem.GetSenseClassForStimulus` (`|GetArrayItem` _lastsensedstimuli_2 1)))
          (set `self.LastSenseClass` _returnvalue_2)
          (`KismetArrayLibrary.Array_AddUnique` _heardactors _array_element)
          (else
            (`KismetArrayLibrary.Array_RemoveItem` _heardactors _array_element))))))
  (`|ExecutionSequence`
    (:`then_0`
      (bind _output_get (set `self.VisibleActors` (`self.VisibleActors`)))
      (for _array_element_2 _output_get
        (`KismetArrayLibrary.Array_AddUnique` _percievedactors _array_element_2)))
    (:`then_1`
      (bind _output_get_2 (set `self.HeardActors` (`self.HeardActors`)))
      (for _array_element_3 _output_get_2
        (`KismetArrayLibrary.Array_AddUnique` _percievedactors _array_element_3)))
    (:`then_2`
      (set `self.LastSenseClass` (`self.LastSenseClass`))
      (return))))

(fn `UpdateInfo`
  (set `self.PlayerVisibility` (`/Game/Player/Blueprints/Banished_Player.Visibility` (`self.Player`)))
  (set `/Game/AI/Blueprints/Banished_AI_Character.Current AI State` (cast `/Game/AI/Blueprints/AIState` (`BlackboardComponent.GetValueAsEnum` (`self.Blackboard`) "AIState")) (`self.ControlledPawn`))
  (bind _output_get (set `self.Veil Strength` (`/Game/Global/Framework/Banished_GameState.Veil Strength` (`self.GameState`))))
  (`BlackboardComponent.SetValueAsFloat` (`self.Blackboard`) "VeilStrength" _output_get)
  (return))

(fn `UserConstructionScript`)