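; Cover is an environment Blueprint that tells Banished_Player when it enters or leaves a cover area.
; Overlap begin and end events on its Cover component add or remove the Blueprint instance in the player's ActiveCovers list, skipping dead players.
; After each change it calls the player's SetInCover, leaving the cover state itself to the player.
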(event `self.Cover.OnComponentBeginOverlap`
  (params (OverlappedComponent :type "PrimitiveComponent Object Reference") (OtherActor :type "Actor Object Reference") (OtherComp :type "PrimitiveComponent Object Reference") (OtherBodyIndex :type Integer) (bFromSweep :type Boolean) (SweepResult :type "HitResult Structure (by ref)"))
  (bind _asbanished_player (cast `/Game/Player/Blueprints/Banished_Player` OtherActor))
  (if (not (`/Game/Player/Blueprints/Banished_Player.Dead` _asbanished_player))
    (`KismetArrayLibrary.Array_AddUnique` (`/Game/Player/Blueprints/Banished_Player.Active Covers` _asbanished_player) self)
    (`/Game/Player/Blueprints/Banished_Player.Set In Cover` _asbanished_player)))

(event `self.Cover.OnComponentEndOverlap`
  (params (OverlappedComponent :type "PrimitiveComponent Object Reference") (OtherActor :type "Actor Object Reference") (OtherComp :type "PrimitiveComponent Object Reference") (OtherBodyIndex :type Integer))
  (bind _asbanished_player (cast `/Game/Player/Blueprints/Banished_Player` OtherActor))
  (if (not (`/Game/Player/Blueprints/Banished_Player.Dead` _asbanished_player))
    (`KismetArrayLibrary.Array_RemoveItem` (`/Game/Player/Blueprints/Banished_Player.Active Covers` _asbanished_player) self)
    (`/Game/Player/Blueprints/Banished_Player.Set In Cover` _asbanished_player)))

(fn `UserConstructionScript`)