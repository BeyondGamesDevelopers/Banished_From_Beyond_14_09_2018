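; Openable gate actor that raises from its starting location by OpenAmount when activated and lowers back when deactivated.
; BeginPlay caches the initial location, and the Activate event plays audio, then plays or reverses the GateOpening timeline.
; Timeline updates set the actor's Z without sweeping, selecting an ease-in-out curve for opening and an inverted ease-in curve for closing.
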(event `self.ReceiveBeginPlay`
  ;[0 1 0] Gate Function
  (set `self.Initial Gate Location` (`self.K2_GetActorLocation`)))

(event `/Game/Interactables/BPI_Activate.Activate`
  (params (Activated :type Boolean) (Instigator :type "Actor Object Reference"))
  (bind _open_amount (`self.Open Amount`))
  ;[0 1 0] Gate Function
  (`AudioComponent.Play` (`self.Audio`) 0.0)
  (if Activated
    (bind (_direction _gate_opening) (`Timeline|Gate Opening` :!label _label)
      (:`Update`
        (`self.K2_SetActorLocation` (`KismetMathLibrary.MakeVector` (.x (`self.Initial Gate Location`)) (.y (`self.Initial Gate Location`)) (+ (.z (`self.Initial Gate Location`)) (`KismetMathLibrary.SelectFloat` (`|EaseFunction` "EaseInOut" _gate_opening 0.0 _open_amount 2.0) (`|EaseFunction` "EaseIn" (`KismetMathLibrary.InverseLerp` 1.0 0.0 _gate_opening) _open_amount 0.0 2.0) Activated))))))
    (else
      (goto _label :!via `Reverse`))))

(fn `UserConstructionScript`)