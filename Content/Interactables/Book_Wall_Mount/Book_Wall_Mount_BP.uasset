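; Book wall mount interactable, marked WIP, that sets the player's Clarity to 1.0 when used.
; A box overlap adds and removes it from Banished_Player's GenericInteractables list.
; Interact disables input, uses SimpleMoveToLocation toward a point behind the mount's forward vector, waits a fixed delay, plays the Killed_Heaven sound, sets Clarity, then restores input.
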(event `/Game/Interactables/BPI_Interact.Interact`
  (params (Instigator :type "Pawn Object Reference") (`Interactable Actor` :type "Actor Object Reference"))
  (bind _returnvalue (`GameplayStatics.GetPlayerController` 0))
  ;[1 0 0] WIP
  (`self.DisableInput` Instigator _returnvalue)
  (`NavigationSystem.SimpleMoveToLocation` _returnvalue (+ (`self.K2_GetActorLocation`) (* (`KismetMathLibrary.GetForwardVector` (`self.K2_GetActorRotation`)) -100.0)))
  (`KismetSystemLibrary.Delay` 2.0)
  (`GameplayStatics.PlaySound2D` "/Game/AI/Audio/Killed/Killed_Heaven.Killed_Heaven")
  (set `/Game/Player/Blueprints/Banished_Player.Clarity` 1.0 (cast `/Game/Player/Blueprints/Banished_Player` Instigator :!pure true))
  (`self.EnableInput` _returnvalue _returnvalue)
  (`self.EnableInput` Instigator _returnvalue))

(event `self.Box Collision.OnComponentBeginOverlap`
  (params (OverlappedComponent :type "PrimitiveComponent Object Reference") (OtherActor :type "Actor Object Reference") (OtherComp :type "PrimitiveComponent Object Reference") (OtherBodyIndex :type Integer) (bFromSweep :type Boolean) (SweepResult :type "HitResult Structure (by ref)"))
  ;[0 1 0] Update As Generic Interactable
  (bind _asbanished_player (cast `/Game/Player/Blueprints/Banished_Player` OtherActor))
  (`KismetArrayLibrary.Array_AddUnique` (`/Game/Player/Blueprints/Banished_Player.Generic Interactables` _asbanished_player) self))

(event `self.Box Collision.OnComponentEndOverlap`
  (params (OverlappedComponent :type "PrimitiveComponent Object Reference") (OtherActor :type "Actor Object Reference") (OtherComp :type "PrimitiveComponent Object Reference") (OtherBodyIndex :type Integer))
  ;[0 1 0] Update As Generic Interactable
  (bind _asbanished_player (cast `/Game/Player/Blueprints/Banished_Player` OtherActor))
  (`KismetArrayLibrary.Array_RemoveItem` (`/Game/Player/Blueprints/Banished_Player.Generic Interactables` _asbanished_player) self))

(fn `UserConstructionScript`
  (`parent.UserConstructionScript`))