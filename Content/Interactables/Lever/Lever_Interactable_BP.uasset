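; Interactable lever that toggles between activated and deactivated, swinging its handle with an audio cue.
; Interact passes a DoOnce into a FlipFlop that plays or reverses a timeline, rolling the handle from its initial rotation with direction-dependent easing.
; When the timeline finishes, it sets Activated from the end position and sends it to Target through BPI_Activate, with debug prints.
; Unless SingleUse is set, a short delay then re-arms the lever.
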(event `self.ReceiveBeginPlay`
  ;[0 1 0] Lever Interaction
  (set `self.InitialLeverRotation` (`SceneComponent.K2_GetComponentRotation` (`self.Lever_Handle`))))

(event `/Game/Interactables/BPI_Interact.Interact`
  (params (Instigator :type "Pawn Object Reference") (`Interactable Actor` :type "Actor Object Reference"))
  ;[0 1 0] Lever Interaction
  (`/Engine/EditorBlueprintResources/StandardMacros.DoOnce` false :!label _label
    (:`Completed`
      (`AudioComponent.Play` (`self.Audio`) 0.0)
      (bind _isa (`/Engine/EditorBlueprintResources/StandardMacros.FlipFlop`)
        (:`A`
          (bind (_direction _lever_direction) (`Timeline|Lever_Direction` :!label _label_2)
            (:`Update`
              (`SceneComponent.K2_SetWorldRotation` (`self.Lever_Handle`) (`KismetMathLibrary.MakeRotator` (+ (.roll (`self.InitialLeverRotation`)) (`KismetMathLibrary.SelectFloat` (`|EaseFunction` "EaseIn" _lever_direction 0.0 50.0 7.0) (`|EaseFunction` "EaseIn" (`KismetMathLibrary.InverseLerp` 1.0 0.0 _lever_direction) 50.0 0.0 7.0) _isa)) (.pitch (`self.InitialLeverRotation`)) (.yaw (`self.InitialLeverRotation`))) false false))
            (:`Finished`
              (`|ExecutionSequence`
                (:`then_0`
                  (if (`KismetMathLibrary.NearlyEqual_FloatFloat` _lever_direction 1.0 0.001)
                    (set `self.Activated` true)
                    ;[1 0 1] DEBUG
                    (`KismetSystemLibrary.PrintString` "Lever Is Activated..." true true (struct :`G` 1.0 :`A` 1.0))
                    (else
                      (set `self.Activated` false)
                      (`KismetSystemLibrary.PrintString` "Lever Is Disactivated..." true true (struct :`R` 1.0 :`G` 0.146921 :`A` 1.0)))))
                (:`then_1`
                  (if (`KismetSystemLibrary.DoesImplementInterface` (`self.Target`) "/Game/Interactables/BPI_Activate.BPI_Activate_C")
                    (message `/Game/Interactables/BPI_Activate.Activate` (`self.Target`) (`self.Activated`) self)
                    (`KismetSystemLibrary.PrintString` "ACTIVATION SENT TO TARGET" true true (struct :`G` 1.0 :`B` 0.535759 :`A` 1.0))
                    (else
                      (`KismetSystemLibrary.PrintString` "ACTIVATION FAILED" true true (struct :`R` 1.0 :`G` 0.10736 :`A` 1.0)))))
                (:`then_2`
                  (if (not (`self.Single Use`))
                    (`KismetSystemLibrary.RetriggerableDelay` 1.0)
                    (goto _label :!via `Reset`)))))))
        (:`B`
          (goto _label_2 :!via `Reverse`))))))

(fn `UserConstructionScript`
  (`parent.UserConstructionScript`))