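; Player scent actor that lets Banished AI characters perceive the player by smell through an overlap sphere.
; Each tick it matches the sphere and particle scale to the player's scent radius, collapsing to zero during possession.
; Overlaps track living AIs and set their blackboard scent flag.
; Tick writes a capped, distance-based linear strength to each tracked blackboard, clearing and dropping dead AIs.
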(event `self.ReceiveBeginPlay`
  ;[0 1 0] Begin Play
  (bind _asbanished_game_mode (cast `/Game/Global/Framework/Banished_GameMode` (`GameplayStatics.GetGameMode`)))
  (set `self.Player` (`/Game/Global/Framework/Banished_GameMode.Player` _asbanished_game_mode)))

(event `self.ReceiveTick`
  (params (DeltaSeconds :type "Float (single-precision)"))
  ;[0 1 0] Tick
  (`self.Update Scent Radius`)
  (`self.Update Percieved Player Scent Amount`))

(event `self.ReceiveActorBeginOverlap`
  (params (OtherActor :type "Actor Object Reference"))
  ;[0 1 0] Update AIs In Range
  (bind _asbanished_ai_character (cast `/Game/AI/Blueprints/Banished_AI_Character` OtherActor))
  (if (not (`/Game/AI/Blueprints/Banished_AI_Character.IsDead` _asbanished_ai_character))
    (`BlackboardComponent.SetValueAsBool` (`AIBlueprintHelperLibrary.GetBlackboard` (`/Game/AI/Blueprints/Banished_AI_Character.Banished_AI_Controller` _asbanished_ai_character)) "PercievedPlayerScent" true)
    (`KismetArrayLibrary.Array_AddUnique` (`self.AIsInRadius`) _asbanished_ai_character)))

(event `self.ReceiveActorEndOverlap`
  (params (OtherActor :type "Actor Object Reference"))
  ;[0 1 0] Update AIs In Range
  (bind _asbanished_ai_character (cast `/Game/AI/Blueprints/Banished_AI_Character` OtherActor))
  (if (not (`/Game/AI/Blueprints/Banished_AI_Character.IsDead` _asbanished_ai_character))
    (bind _returnvalue (`AIBlueprintHelperLibrary.GetBlackboard` (`/Game/AI/Blueprints/Banished_AI_Character.Banished_AI_Controller` _asbanished_ai_character)))
    (`BlackboardComponent.SetValueAsBool` _returnvalue "PercievedPlayerScent" false)
    (`BlackboardComponent.SetValueAsFloat` _returnvalue "PercievedPlayerScentAmount" 0.0)
    (`KismetArrayLibrary.Array_RemoveItem` (`self.AIsInRadius`) _asbanished_ai_character)))

(fn `Update Percieved Player Scent Amount`
  (for _array_element (`self.AIsInRadius`)
    (if (not (`/Game/AI/Blueprints/Banished_AI_Character.IsDead` _array_element))
      (bind _returnvalue (`AIBlueprintHelperLibrary.GetBlackboard` (`AIBlueprintHelperLibrary.GetAIController` _array_element)))
      (`BlackboardComponent.SetValueAsFloat` _returnvalue "PercievedPlayerScentAmount" (`KismetMathLibrary.FClamp` (* (`KismetMathLibrary.FClamp` (`KismetMathLibrary.Lerp` 1.0 0.0 (`KismetMathLibrary.NormalizeToRange` (`self.GetDistanceTo` _array_element) 0.0 (`.SphereRadius` (`KismetSystemLibrary.GetComponentBounds` (`self.Scent Collision`)))))) 0.65) 0.0 1.0))
      (else
        (`BlackboardComponent.SetValueAsBool` _returnvalue "PercievedPlayerScent" false)
        (`BlackboardComponent.SetValueAsFloat` _returnvalue "PercievedPlayerScentAmount" 0.0)
        (`KismetArrayLibrary.Array_RemoveItem` (`self.AIsInRadius`) _array_element)))))

(fn `Update Scent Radius`
  (bind _scent_collision (`self.Scent Collision`))
  (bind _player (`self.Player`))
  (bind _sphereradius (`SphereComponent.SphereRadius` _scent_collision))
  (`SphereComponent.SetSphereRadius` _scent_collision (`KismetMathLibrary.SelectFloat` 0.0 (`/Game/Player/Blueprints/Banished_Player.Scent Radius` _player) (`/Game/Player/Blueprints/Banished_Player.Using Possession` _player)) true)
  (`SceneComponent.SetWorldScale3D` (`self.Scent_ParticleSystem`) (`KismetMathLibrary.MakeVector` _sphereradius _sphereradius _sphereradius)))

(fn `UserConstructionScript`)