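; Noise effect actor that shows a player noise as a sphere expanding from zero toward a target radius, then destroys itself.
; Tick interpolates the scale, using a delta-time helper that can apply the player's custom time dilation.
; An expansion-alpha check at or below 0.75 triggers a one-shot opacity timeline that destroys the actor when finished.
; A one-second timer also destroys it, covering a stray sphere at initial player spawn.
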(event `self.ReceiveBeginPlay`
  (`SceneComponent.SetWorldScale3D` (`self.Sphere`) (0.0 0.0 0.0))
  (`MeshComponent.SetScalarParameterValueOnMaterials` (`self.Sphere`) "Opacity" (`self.Opacity`))
  (bind _asbanished_game_mode (cast `/Game/Global/Framework/Banished_GameMode` (`GameplayStatics.GetGameMode`)))
  (set `self.Player` (`/Game/Global/Framework/Banished_GameMode.Player` _asbanished_game_mode))
  (`KismetSystemLibrary.K2_SetTimerDelegate` (delegate `Destroy`) 1.0) ; Time Equal To Opacity Fade Timeline Length,\nThis Destroy Event Is Used On The Occasion\nWhere Initial Spawing Player Makes Noise Sphere\nThat Doesn't Get Destroyed.
)

(event `Destroy`
  (`self.K2_DestroyActor`))

(event `self.ReceiveTick`
  (params (DeltaSeconds :type "Float (single-precision)"))
  (bind _output_get (set `self.Radius` (`KismetMathLibrary.VInterpTo` (`SceneComponent.K2_GetComponentScale` (`self.Sphere`)) (`self.TargetRadius`) (`self.Get World Delta Seconds`) 17.0)))
  (`SceneComponent.SetWorldScale3D` (`self.Sphere`) _output_get)
  (if (<= (`self.Get Expansion Alpha`) 0.75)
    (`/Engine/EditorBlueprintResources/StandardMacros.DoOnce` false
      (:`Completed`
        (bind (_direction _opacity_fade) (`Timeline|NoiseOpacityFade` :!via `PlayFromStart`)
          (:`Update`
            (`MeshComponent.SetScalarParameterValueOnMaterials` (`self.Sphere`) "Opacity" (* _opacity_fade 0.75)))
          (:`Finished`
            (`self.K2_DestroyActor`)))))))

(fn `UserConstructionScript`)