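; Transitional pawn that animates the camera during possession, moving it to the third-person camera of the target AI or player character.
; CharacterPossession copies post-process settings and runs an eased timeline with camera shake and force feedback.
; Tick re-runs BeginPlay logic to track the target, hide from AI sight and reverse the timeline if the AI dies.
; On finish it possesses the target, or the reappearing player if dead, then destroys itself.
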(event `Possession`
  (bind _isdead (`/Game/AI/Blueprints/Banished_AI_Character.IsDead` (cast `/Game/AI/Blueprints/Banished_AI_Character` (stale `/Game/Player/Blueprints/BPI_Possession.CharacterPossession` `Possessed Character`) :!pure true)))
  (if _isdead
    (`/Game/Player/Blueprints/Banished_Player.Possession Reappear` (`self.Player`)))
  (`Controller.Possess` (`self.GetController` (`GameplayStatics.GetPlayerPawn` 0)) (select `bool` _isdead :`false` (stale `/Game/Player/Blueprints/BPI_Possession.CharacterPossession` `Possessed Character`) :`true` (`self.Player`) :!type "Pawn Object Reference"))
  (set `self.Camera` null)
  (set `self.CurrentCameraComponent` null)
  (`AIPerceptionStimuliSourceComponent.UnregisterFromSense` (`self.AIPerceptionStimuliSource`) "/Script/AIModule.AISense_Sight")
  (`self.K2_DestroyActor`))

(event `self.ReceivePossessed`
  (params (NewController :type "Controller Object Reference"))
  (bind _asbanished_game_mode (cast `/Game/Global/Framework/Banished_GameMode` (`GameplayStatics.GetGameMode`)))
  (set `self.Player` (`/Game/Global/Framework/Banished_GameMode.Player` _asbanished_game_mode)))

(event `/Game/Player/Blueprints/BPI_Possession.CharacterPossession`
  (params (Instigator :type "Pawn Object Reference") (`Camera Component` :type "CameraComponent Object Reference") (`Possessed Character` :type "Pawn Object Reference") (`Possessing AI` :type Boolean))
  (bind _returnvalue (`GameplayStatics.GetPlayerController` 0))
  (bind _camera (`self.Camera`))
  (set `self.InstigatorPawn` Instigator)
  (bind _output_get (set `self.CurrentCameraComponent` `Camera Component`))
  (set `CameraComponent.PostProcessSettings` (`CameraComponent.PostProcessSettings` _output_get) (`self.Camera`))
  (set `self.PossessingAI` `Possessing AI`)
  (set `self.A_WorldLocation` (`SceneComponent.K2_GetComponentLocation` _camera))
  (set `self.A_WorldRotation` (`SceneComponent.K2_GetComponentRotation` _camera))
  (bind (_direction _path) (`Timeline|PossessionAlpha` :!via `PlayFromStart` :!label _label)
    (:`Update`
      (`SceneComponent.K2_SetWorldLocationAndRotation` (`self.Camera`) (`|EaseFunction` "EaseInOut" _path (`self.A_WorldLocation`) (`self.B_WorldLocation`) 6.0) (`|EaseFunction` "EaseInOut" _path (`self.A_WorldRotation`) (`self.B_WorldRotation`) true 6.0) false true)
      (`PlayerController.ClientStartCameraShake` :`self` _returnvalue :`Shake` "/Game/Player/Camera_Shakes/Possession_Shake.Possession_Shake_C" :`Scale` _path)
      (`/Engine/EditorBlueprintResources/StandardMacros.DoOnce` false
        (:`Completed`
          (`PlayerController.ClientPlayForceFeedback` _returnvalue "/Game/Player/Force_Feedback/Heaven_Kill.Heaven_Kill" false "None"))))
    (:`Finished`
      (`self.Possession`))))

(event `self.ReceiveBeginPlay`
  (bind _possessingai (`self.PossessingAI`))
  (`AIPerceptionStimuliSourceComponent.UnregisterFromSense` (`self.AIPerceptionStimuliSource`) "/Script/AIModule.AISense_Sight" :!label _label_2)
  (`|ExecutionSequence`
    (:`then_0`
      (if (`/Game/AI/Blueprints/Banished_AI_Character.IsDead` (cast `/Game/AI/Blueprints/Banished_AI_Character` (stale `/Game/Player/Blueprints/BPI_Possession.CharacterPossession` `Possessed Character`) :!pure true))
        (goto _label :!via `Reverse`)))
    (:`then_1`
      (`|ExecutionSequence`
        (:`then_0`
          (bind _thirdpersoncamera (`/Game/AI/Blueprints/Banished_AI_Character.ThirdPersonCamera` (cast `/Game/AI/Blueprints/Banished_AI_Character` (stale `/Game/Player/Blueprints/BPI_Possession.CharacterPossession` `Possessed Character`) :!pure true)))
          (bind _thirdpersoncamera_2 (`/Game/Player/Blueprints/Banished_Player.ThirdPersonCamera` (cast `/Game/Player/Blueprints/Banished_Player` (stale `/Game/Player/Blueprints/BPI_Possession.CharacterPossession` `Possessed Character`) :!pure true)))
          (set `self.B_WorldLocation` (`KismetMathLibrary.SelectVector` (`SceneComponent.K2_GetComponentLocation` _thirdpersoncamera) (`SceneComponent.K2_GetComponentLocation` _thirdpersoncamera_2) _possessingai)))
        (:`then_1`
          (set `self.B_WorldRotation` (`KismetMathLibrary.SelectRotator` (`SceneComponent.K2_GetComponentRotation` _thirdpersoncamera) (`SceneComponent.K2_GetComponentRotation` _thirdpersoncamera_2) _possessingai))))
      ;[1 0 1] DEBUG
      (`KismetSystemLibrary.PrintString` "PLAYING AS POSSESSING PAWN..." true true (struct :`G` 1.0 :`A` 1.0) 0.005))))

(event `self.ReceiveTick`
  (params (DeltaSeconds :type "Float (single-precision)"))
  (goto _label_2))

(fn `UserConstructionScript`)