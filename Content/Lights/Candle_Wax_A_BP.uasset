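; Wax candle light Blueprint with seven flames that can be blown out.
; BlowLight stores the Blown state, calls LightBlown and plays the CandleDim timeline, which drives the light intensity and the Opacity material parameter on wax and flames.
; The light lerps from zero to its current intensity each update, so dimming compounds.
; When the timeline finishes, the light and flame components are destroyed, leaving the wax.
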(event `self.ReceiveTick`
  (params (DeltaSeconds :type "Float (single-precision)"))
  (`parent.ReceiveTick` DeltaSeconds))

(event `/Game/Interactables/BPI_Blowable.BlowLight`
  (params (Instigator :type "Pawn Object Reference") (Blown :type Boolean))
  (set `self.Blown` Blown)
  (`self.Light Blown`)
  (bind (_direction _candledim) (`Timeline|CandleDim`)
    (:`Update`
      (`self.DimLight` (`self.TraceLight`) _candledim)
      (`self.UpdateCandleEmissive` (`self.Candle_Wax_A`) _candledim)
      (`self.DimFlame` (`self.Flame1`) _candledim)
      (`self.DimFlame` (`self.Flame2`) _candledim)
      (`self.DimFlame` (`self.Flame3`) _candledim)
      (`self.DimFlame` (`self.Flame4`) _candledim)
      (`self.DimFlame` (`self.Flame5`) _candledim)
      (`self.DimFlame` (`self.Flame6`) _candledim)
      (`self.DimFlame` (`self.Flame7`) _candledim))
    (:`Finished`
      (`ActorComponent.K2_DestroyComponent` (`self.TraceLight`))
      (`ActorComponent.K2_DestroyComponent` (`self.Flame1`))
      (`ActorComponent.K2_DestroyComponent` (`self.Flame2`))
      (`ActorComponent.K2_DestroyComponent` (`self.Flame3`))
      (`ActorComponent.K2_DestroyComponent` (`self.Flame4`))
      (`ActorComponent.K2_DestroyComponent` (`self.Flame5`))
      (`ActorComponent.K2_DestroyComponent` (`self.Flame6`))
      (`ActorComponent.K2_DestroyComponent` (`self.Flame7`)))))

(fn `DimFlame`
  (params (Target :type "MeshComponent Object Reference") (Alpha :type "Float (double-precision)"))
  (`MeshComponent.SetScalarParameterValueOnMaterials` Target "Opacity" (* Alpha 15.0)))

(fn `DimLight`
  (params (Target :type "LightComponent Object Reference") (Alpha :type "Float (double-precision)"))
  (`LightComponent.SetIntensity` Target (`KismetMathLibrary.Lerp` 0.0 (`LightComponentBase.Intensity` Target) Alpha)))

(fn `UpdateCandleEmissive`
  (params (Target :type "MeshComponent Object Reference") (Alpha :type "Float (double-precision)"))
  (`MeshComponent.SetScalarParameterValueOnMaterials` Target "Opacity" (* Alpha 0.5)))

(fn `UserConstructionScript`
  (`parent.UserConstructionScript`))