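; Votive candle light Blueprint that can be blown out, fading its flame and lights.
; The construction script copies attenuation radius, intensity and color from TraceLight to two point lights.
; BlowLight calls LightBlown and plays the CandleDim timeline, driving the candle materials' Opacity and all three light intensities, then destroys the lights.
; DimLight lerps from each light's current intensity, so dimming compounds per update.
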(event `self.ReceiveTick`
  (params (DeltaSeconds :type "Float (single-precision)"))
  (`parent.ReceiveTick` DeltaSeconds))

(event `/Game/Interactables/BPI_Blowable.BlowLight`
  (params (Instigator :type "Pawn Object Reference") (Blown :type Boolean))
  (set `self.Blown` Blown)
  (`self.Light Blown`)
  (bind (_direction _candledim) (`Timeline|CandleDim`)
    (:`Update`
      (`self.UpdateCandleEmissive` (`self.Votive_Candle_B`) _candledim)
      (`self.DimLight` (`self.TraceLight`) _candledim)
      (`self.DimLight` (`self.PointLight`) _candledim)
      (`self.DimLight` (`self.PointLight_2`) _candledim))
    (:`Finished`
      (`ActorComponent.K2_DestroyComponent` (`self.TraceLight`))
      (`ActorComponent.K2_DestroyComponent` (`self.PointLight`))
      (`ActorComponent.K2_DestroyComponent` (`self.PointLight_2`)))))

(fn `DimLight`
  (params (Target :type "LightComponent Object Reference") (Alpha :type "Float (double-precision)"))
  (`LightComponent.SetIntensity` Target (`KismetMathLibrary.Lerp` 0.0 (`LightComponentBase.Intensity` Target) Alpha)))

(fn `UpdateCandleEmissive`
  (params (Target :type "MeshComponent Object Reference") (Alpha :type "Float (double-precision)"))
  (`MeshComponent.SetScalarParameterValueOnMaterials` Target "Opacity" (* Alpha 0.5)))

(fn `UserConstructionScript`
  (bind _pointlight (`self.PointLight`))
  (bind _tracelight (`self.TraceLight`))
  (bind _pointlight_2 (`self.PointLight_2`))
  (bind _returnvalue (`LightComponentBase.GetLightColor` _tracelight))
  (bind _attenuationradius (`PointLightComponent.AttenuationRadius` _tracelight))
  (bind _intensity (`LightComponentBase.Intensity` _tracelight))
  (`parent.UserConstructionScript`)
  (`PointLightComponent.SetAttenuationRadius` _pointlight _attenuationradius)
  (`LightComponent.SetIntensity` _pointlight _intensity)
  (`LightComponent.SetLightColor` _pointlight _returnvalue true)
  (`PointLightComponent.SetAttenuationRadius` _pointlight_2 _attenuationradius)
  (`LightComponent.SetIntensity` _pointlight_2 _intensity)
  (`LightComponent.SetLightColor` _pointlight_2 _returnvalue true))