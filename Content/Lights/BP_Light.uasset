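; Light actor that computes how brightly it lights the player, as a Brightness value.
; Its attenuation-sized sphere registers it in player and AI nearby-light lists (plus EQS lists if tagged) and enables Tick for the player.
; Tick traces to each player bone socket, scaling the hit fraction by UE4-style distance falloff and a multiplier.
; LightBlown zeroes Brightness, destroys the sphere and briefly registers an AI perception stimulus.
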(event OnComponentBeginOverlap(Sphere)
  (params (OverlappedComponent :type Primitive%20Component%20Object%20Reference) (OtherActor :type Actor%20Object%20Reference) (OtherComp :type Primitive%20Component%20Object%20Reference) (OtherBodyIndex :type Integer) (bFromSweep :type Boolean) (SweepResult :type Hit%20Result%20Structure%20%28by%20ref%29))
  (bind _self self)
  ;[0 1 0] Adds And Removes the Lights Array From The Player & AI Characters, Controls Tick
  (Utilities|FlowControl|Sequence
    (:then_0
      (bind _asbanished_player (Utilities|Casting|CastToBanished_Player OtherActor))
      (Utilities|Array|AddUnique (Variables|/Game/Player/Blueprints/Banished_Player.Banished_Player_C|GetNearby%20Lights _asbanished_player) _self)
      (Variables|Default|SetPlayer _asbanished_player)
      (Actor|Tick|SetActorTickEnabled true))
    (:then_1
      (bind _asbanished_ai_character (Utilities|Casting|CastToBanished_AI_Character OtherActor))
      (Utilities|Array|AddUnique (Variables|/Game/AI/Blueprints/Banished_AI_Character.Banished_AI_Character_C|GetNearby%20Lights _asbanished_ai_character) _self)
      (if (Actor|ActorHasTag "EQS Light")
        (Utilities|Array|AddUnique (Variables|/Game/AI/Blueprints/Banished_AI_Character.Banished_AI_Character_C|GetEQS%20Lights _asbanished_ai_character) self)))))

(event OnComponentEndOverlap(Sphere)
  (params (OverlappedComponent :type Primitive%20Component%20Object%20Reference) (OtherActor :type Actor%20Object%20Reference) (OtherComp :type Primitive%20Component%20Object%20Reference) (OtherBodyIndex :type Integer))
  (bind _self self)
  ;[0 1 0] Adds And Removes the Lights Array From The Player & AI Characters, Controls Tick
  (Utilities|FlowControl|Sequence
    (:then_0
      (bind _asbanished_player (Utilities|Casting|CastToBanished_Player OtherActor))
      (Utilities|Array|RemoveItem (Variables|/Game/Player/Blueprints/Banished_Player.Banished_Player_C|GetNearby%20Lights _asbanished_player) _self)
      (Actor|Tick|SetActorTickEnabled false)
      (Variables|Default|SetPlayer 0)
      (Variables|Default|SetBrightness 0.0))
    (:then_1
      (bind _asbanished_ai_character (Utilities|Casting|CastToBanished_AI_Character OtherActor))
      (Utilities|Array|RemoveItem (Variables|/Game/AI/Blueprints/Banished_AI_Character.Banished_AI_Character_C|GetNearby%20Lights _asbanished_ai_character) _self)
      (if (Actor|ActorHasTag "EQS Light")
        (Utilities|Array|RemoveItem (Variables|/Game/AI/Blueprints/Banished_AI_Character.Banished_AI_Character_C|GetEQS%20Lights _asbanished_ai_character) self)))))

(event Custom|Light%20Blown
  (bind _aiperceptionstimulisource (Variables|Default|GetAIPerceptionStimuliSource))
  ;[0 1 0] Light Blown
  (Utilities|FlowControl|DoOnce false
    (:Completed
      (Actor|Tick|SetActorTickEnabled false)
      (Variables|Default|SetBrightness 0.0)
      (Components|DestroyComponent (Variables|Default|GetSphere))
      (Class|AIPerceptionStimuliSourceComponent|RegisterwithPerceptionSystem _aiperceptionstimulisource)
      (Utilities|FlowControl|Delay 1.0)
      (Class|AIPerceptionStimuliSourceComponent|UnregisterfromPerceptionSystem _aiperceptionstimulisource)
      (Development|PrintString (Utilities|String|Append (Utilities|GetDisplayName self) ": " "Blown") true true "(R=1.000000,G=0.505835,B=0.000000,A=1.000000)"))))

(event EventBeginPlay
  ;[0 1 0] Initial Set Up
  (Class|AIPerceptionStimuliSourceComponent|UnregisterfromPerceptionSystem (Variables|Default|GetAIPerceptionStimuliSource))
  (Rendering|Lighting|SetAttenuationRadius (Variables|Default|GetTraceLight) (Variables|LightingSettings|GetAttenuationRadius))
  (Rendering|Components|Light|SetLightColor (Variables|Default|GetTraceLight) (Variables|LightingSettings|GetLightHue) true)
  (Rendering|Components|Light|SetIntensity (Variables|Default|GetTraceLight) (Variables|LightingSettings|GetIntensity))
  (CallFunction|SetSphereRadius))

(event EventTick
  (params (DeltaSeconds :type Float%20%28single-precision%29))
  ;[0 1 0] Calculates Per Bone Visibility For Player, Calculates Visibility Using UE4 Falloff Math
  (bind _keys (Utilities|Map|Keys (Variables|/Game/Player/Blueprints/Banished_Player.Banished_Player_C|GetBoneSockets (Variables|Default|GetPlayer))))
  (for _array_element _keys
    (CallFunction|PerBoneVisibilityTrace _array_element))
  (CallFunction|BoneTraceResultantCalculation))

(fn ConstructionScript
  (bind _tracelight (Variables|Default|GetTraceLight))
  (Rendering|Lighting|SetAttenuationRadius _tracelight (Variables|LightingSettings|GetAttenuationRadius))
  (Rendering|Components|Light|SetLightColor _tracelight (Variables|LightingSettings|GetLightHue) true)
  (Rendering|Components|Light|SetIntensity (Variables|Default|GetTraceLight) (Variables|LightingSettings|GetIntensity))
  (CallFunction|SetSphereRadius))

(fn SetSphereRadius
  (Components|Sphere|SetSphereRadius (Variables|Default|GetSphere) (Variables|/Script/Engine.PointLightComponent|GetAttenuationRadius (Variables|Default|GetTraceLight)) true))

(fn PerBoneVisibilityTrace
  (params (BoneSocket :type Name))
  (bind _outhit (Collision|LineTraceByChannel (Transformation|GetWorldLocation (Variables|Default|GetTraceLight)) (.Value (Utilities|Map|Find (Variables|/Game/Player/Blueprints/Banished_Player.Banished_Player_C|GetBoneSockets (Variables|Default|GetPlayer)) BoneSocket)) "TraceTypeQuery1" true 0 "None"))
  (Utilities|Map|Add (Variables|Default|GetBone%20Trace%20Results) BoneSocket (== (.hitcomponent _outhit) (Variables|/Script/Engine.Character|GetMesh (Variables|Default|GetPlayer))))
  (Variables|Default|SetBone%20Hits (+ (Variables|Default|GetBone%20Hits) (Math|Integer|SelectInt 1 0 (== (.hitcomponent _outhit) (Variables|/Script/Engine.Character|GetMesh (Variables|Default|GetPlayer)))))))

(fn BoneTraceResultantCalculation
  (bind _tracelight (Variables|Default|GetTraceLight))
  (bind _attenuationradius (Variables|/Script/Engine.PointLightComponent|GetAttenuationRadius _tracelight))
  (Variables|Default|SetBone%20Trace%20Results (Variables|Default|GetBone%20Trace%20Results))
  (Variables|Default|SetBone%20Hit%20Alpha (Math|Float|Clamp(Float) (Math|Float|NormalizetoRange (Math|Conversions|ToFloat(Integer) (Variables|Default|GetBone%20Hits)) 0.0 (Math|Conversions|ToFloat(Integer) (Utilities|Map|Length (Variables|Default|GetBone%20Trace%20Results))))))
  (bind _values (Utilities|Map|Values (Variables|Default|GetBone%20Trace%20Results)))
  (if (Utilities|Array|ContainsItem _values true)
    (Variables|Default|SetBrightness (* (|(pow((1-(pow((distance/radius),4))),2)) (Math|Float|Min(Float) (Transformation|GetDistanceTo (Variables|Default|GetPlayer)) _attenuationradius) _attenuationradius) (Variables|Default|GetBone%20Hit%20Alpha) (Variables|LightingSettings|GetVisibility%20Multiplier)))
    (else
      (Variables|Default|SetBrightness 0.0)))
  (Utilities|Map|Clear (Variables|Default|GetBone%20Trace%20Results))
  (Variables|Default|SetBone%20Hits 0)
  (Variables|Default|SetBone%20Hit%20Alpha 0.0))