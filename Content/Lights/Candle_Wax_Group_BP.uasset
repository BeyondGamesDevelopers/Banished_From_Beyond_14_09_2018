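; Candle wax group light Blueprint that dims and goes out when blown.
; The BlowLight event stores the blown state, calls LightBlown, and plays the CandleDim timeline.
; The timeline drives the Opacity material parameter on three wax components and scales TraceLight's intensity.
; Intensity scales from its current value each update, so dimming compounds, and TraceLight is destroyed when the timeline finishes.
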(event `self.ReceiveTick`
  (params (DeltaSeconds :type "Float (single-precision)"))
  (`parent.ReceiveTick` DeltaSeconds))

(event `/Game/Interactables/BPI_Blowable.BlowLight`
  (params (Instigator :type "Pawn Object Reference") (Blown :type Boolean))
  (set `self.Blown` Blown)
  (`self.Light Blown`)
  (bind (_direction _candledim) (`Timeline|CandleDim`)
    (:`Update`
      (`self.UpdateCandleEmissive` (`self.Candle_Wax_B`) _candledim)
      (`self.UpdateCandleEmissive` (`self.Candle_Wax_A`) _candledim)
      (`self.UpdateCandleEmissive` (`self.Candle_Wax_A_2`) _candledim)
      (`self.DimLight` (`self.TraceLight`) _candledim))
    (:`Finished`
      (`ActorComponent.K2_DestroyComponent` (`self.TraceLight`)))))

(fn `DimLight`
  (params (Target :type "LightComponent Object Reference") (Alpha :type "Float (double-precision)"))
  (`LightComponent.SetIntensity` Target (`KismetMathLibrary.Lerp` 0.0 (`LightComponentBase.Intensity` Target) Alpha)))

(fn `UpdateCandleEmissive`
  (params (Target :type "MeshComponent Object Reference") (Alpha :type "Float (double-precision)"))
  (`MeshComponent.SetScalarParameterValueOnMaterials` Target "Opacity" (* Alpha 0.5)))

(fn `UserConstructionScript`
  (`parent.UserConstructionScript`))